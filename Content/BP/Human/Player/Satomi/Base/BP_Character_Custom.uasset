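; Modular customisable character that builds its face, body and outfit look from exposed variables, in both the construction script and BeginPlay.
; ModularSetup slaves part meshes to the main mesh and groups them into body, outfit and hair arrays.
; CustomisationSetup maps signed sliders onto positive/negative morph pairs, then sets skin, eye, hair and cloth material parameters.
; AnimationSetup is empty, and the style-enum mask lookup (SetSkinMasks) is left unconnected.
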(event `self.ReceiveBeginPlay`
  (`parent.ReceiveBeginPlay`)
  (`self.ModularSetup`)
  (`self.AnimationSetup`)
  (`self.CustomisationSetup`))

(fn `AnimationSetup`)

(fn `CustomisationSetup`
  (locals (`Morph Targets` :type "/Game/XANDRA/_Master/Blueprints/Structs/S_CustomCharacter Structure"))
  (bind _m_skin (`self.M_Skin`))
  (bind _outfitcomponents (`self.OutfitComponents`))
  (bind _haircomponents (`self.HairComponents`))
  (bind _m_skin_2 (`self.M_Skin`))
  (bind _lipsize (`self.LipSize`))
  (bind _skincolour (`self.SkinColour`))
  (bind _bodycomponents (`self.BodyComponents`))
  (bind _m_skin_3 (`self.M_Skin`))
  (bind _m_skin_4 (`self.M_Skin`))
  (bind _m_skin_5 (`self.M_Skin`))
  (bind (_bodymale _chestsize _elfears _nosesize _nosewidth _nosetipheight _nostrilsize _jawwidth _chinheight _eyeheight _eyeseperate _cheeksize _cheekbonesize _nosebridgeupperwidth _lipsuppersize _lipslowersize _lipscurve _lipscornerheight _eyelidupperheight _eyelidouterheight _nostrilheight _eyelidcrease) (break `/Game/XANDRA/_Master/Blueprints/Structs/S_CustomCharacter` (`local.Morph Targets`)))
  ;[0.3027 0.8393 1] Set Customisation Morphs
  (`|ExecutionSequence`
    (:`then_0`
      ;;[1 1 1] Other
      ;;;[1 1 1] Elf Ears
      (`self.SetMorphTarget` _elfears (`self.ElfEars`)))
    (:`then_1`
      ;;[1 1 1] Eyes
      ;;;[1 1 1] Eyes Height
      (`self.SetMorphTarget` _eyeheight (`self.EyeHeight`))
      ;;;[1 1 1] Eyes Apart
      (`self.SetMorphTarget` _eyeseperate (`self.EyeSeparation`))
      ;;;[1 1 1] Eye Outer
      (`self.SetMorphTarget` _eyelidouterheight (`self.EyeOuterCornerHeight`))
      ;;;[1 1 1] Eyelid Crease Depth
      (`self.SetMorphTarget` _eyelidcrease (`self.EyelidCreaseDepth`)))
    (:`then_2`
      ;;[1 1 1] Nose
      ;;;[1 1 1] Nose Height
      (`self.SetMorphTarget` (struct) (`self.NoseHeight`))
      ;;;[1 1 1] Nose Width
      (`self.SetMorphTarget` _nosewidth (`self.NoseWidth`))
      ;;;[1 1 1] Nose Tip Height
      (`self.SetMorphTarget` _nosetipheight (`self.NoseTipHeight`))
      ;;;[1 1 1] Nostril Size
      (`self.SetMorphTarget` _nostrilsize (`self.NostrilSize`))
      ;;;[1 1 1] Nostril Height
      (`self.SetMorphTarget` _nostrilheight (`self.NostrilHeight`)))
    (:`then_3`
      ;;[1 1 1] Head Shape
      ;;;[1 1 1] Jaw Width
      (`self.SetMorphTarget` _jawwidth (`self.JawWidth`))
      ;;;[1 1 1] CheekFat
      (`self.SetMorphTarget` _cheeksize (`self.CheekFat`))
      ;;;[1 1 1] CheekboneSize
      (`self.SetMorphTarget` _cheekbonesize (`self.CheekboneSize`))
      ;;[1 1 1] Body
      ;;;[1 1 1] ChestSize
      (`self.SetMorphTarget` _chestsize (`self.ChestSize`))
      ;[1 1 1] Mouth
      ;;[1 1 1] LipSize
      (`self.SetMorphTarget` _lipsuppersize _lipsize)
      (`self.SetMorphTarget` _lipslowersize _lipsize)
      ;;[1 1 1] LipCurve
      (`self.SetMorphTarget` _lipscurve (`self.LipCurve`)))
    (:`then_4`
      (`|ExecutionSequence`
        (:`then_0`
          ;[1 1 1] Set Materials
          ;;[1 1 1] Skin
          (`MeshComponent.SetVectorParameterValueOnMaterials` _bodycomponents "SkinColour" (`KismetMathLibrary.Conv_LinearColorToVector` (`KismetMathLibrary.Conv_ColorToLinearColor` _skincolour)))
          (`MeshComponent.SetVectorParameterValueOnMaterials` _bodycomponents "NailsColour" (`KismetMathLibrary.Conv_LinearColorToVector` (`KismetMathLibrary.Conv_ColorToLinearColor` (`self.NailsColour`))))
          (bind _returnvalue (`PrimitiveComponent.CreateDynamicMaterialInstance` (`self.Mesh`) 0 (`self.Skin Material`) "None"))
          (bind _output_get (set `self.M_Skin` _returnvalue))
          (`MaterialInstanceDynamic.SetVectorParameterValue` _output_get "SkinColour" (`KismetMathLibrary.Conv_ColorToLinearColor` _skincolour))
          (`MaterialInstanceDynamic.SetVectorParameterValue` _m_skin_2 "EyeMakeupColour_A" (`KismetMathLibrary.Conv_ColorToLinearColor` (`self.EyeMakeupColourA`)))
          ;;;[1 1 1] Eye Makeup
          (`MaterialInstanceDynamic.SetVectorParameterValue` _m_skin_2 "EyeMakeupColour_B" (`KismetMathLibrary.Conv_ColorToLinearColor` (`self.EyeMakeupColourB`)))
          (`MaterialInstanceDynamic.SetTextureParameterValue` _m_skin_2 "EyeMakeupMask" (`self.EyeMakeupMask`))
          (`MaterialInstanceDynamic.SetScalarParameterValue` _m_skin_2 "EyeMakeupAmount" (`self.EyeMakeupAmount`))
          (`MaterialInstanceDynamic.SetTextureParameterValue` _m_skin_3 "T_Skin_DIFF" (`self.SkinTextureMain`))
          (`MaterialInstanceDynamic.SetTextureParameterValue` _m_skin_3 "T_Skin_NRM" (`self.SkinNormalMap`))
          (`MaterialInstanceDynamic.SetTextureParameterValue` _m_skin_3 "T_Foundation_DIFF" (`self.FoundationTextureMain`))
          (`MaterialInstanceDynamic.SetScalarParameterValue` _m_skin "FoundationAmount" (`self.FoundationAmount`))
          (`MaterialInstanceDynamic.SetVectorParameterValue` _m_skin "BrowColour" (`KismetMathLibrary.Conv_ColorToLinearColor` (`self.BrowsColour`)))
          (`MaterialInstanceDynamic.SetTextureParameterValue` _m_skin "BrowsMask" (`self.BrowsMask`))
          (`MaterialInstanceDynamic.SetVectorParameterValue` _m_skin "LipColour" (`KismetMathLibrary.Conv_ColorToLinearColor` (`self.LipColour`)))
          (`MaterialInstanceDynamic.SetScalarParameterValue` _m_skin "LipRoughness" (`self.LipRoughness`))
          (`MaterialInstanceDynamic.SetScalarParameterValue` _m_skin "LipstickAmount" (`self.LipstickAmount`))
          ;;;[1 1 1] Blush
          (`MaterialInstanceDynamic.SetVectorParameterValue` _m_skin_4 "BlushColour" (`KismetMathLibrary.Conv_ColorToLinearColor` (`self.BlushColour`)))
          (`MaterialInstanceDynamic.SetTextureParameterValue` _m_skin_4 "BlushMask" (`self.BlushMask`))
          (`MaterialInstanceDynamic.SetScalarParameterValue` _m_skin_4 "BlushAmount" (`self.BlushAmount`))
          ;;;[1 1 1] Freckles
          (`MaterialInstanceDynamic.SetTextureParameterValue` _m_skin_5 "FrecklesMask" (`self.FrecklesMask`))
          (`MaterialInstanceDynamic.SetScalarParameterValue` _m_skin_5 "FrecklesAmount" (`self.FrecklesAmount`))
          (`MaterialInstanceDynamic.SetVectorParameterValue` _m_skin_5 "NailsColour" (`KismetMathLibrary.Conv_ColorToLinearColor` (`self.NailsColour`))))
        (:`then_1`
          ;;[1 1 1] Hair
          (`MeshComponent.SetVectorParameterValueOnMaterials` _haircomponents "HairBaseColour" (`KismetMathLibrary.Conv_LinearColorToVector` (`KismetMathLibrary.Conv_ColorToLinearColor` (`self.HairBaseColour`))))
          (`MeshComponent.SetScalarParameterValueOnMaterials` _haircomponents "HairScatter" (`self.HairScatter`))
          (`MeshComponent.SetScalarParameterValueOnMaterials` _haircomponents "HairHighlightAmount" (`self.HairHighlightAmount`))
          (`MeshComponent.SetVectorParameterValueOnMaterials` _haircomponents "HairHighlightColour" (`KismetMathLibrary.Conv_LinearColorToVector` (`KismetMathLibrary.Conv_ColorToLinearColor` (`self.HairHighlightColour`))))
          (`MeshComponent.SetScalarParameterValueOnMaterials` _haircomponents "HairRoughness" (`self.HairRoughness`)))
        (:`then_2`
          ;;[1 1 1] Eyes
          (bind _returnvalue_2 (`PrimitiveComponent.CreateDynamicMaterialInstance` (`self.Mesh`) 1 (`self.Eyes Mat`) "None"))
          (bind _output_get_2 (set `self.M_Eyes` _returnvalue_2))
          (`MaterialInstanceDynamic.SetVectorParameterValue` _output_get_2 "EyeColour" (`KismetMathLibrary.Conv_ColorToLinearColor` (`self.EyeColour`)))
          (`MaterialInstanceDynamic.SetScalarParameterValue` _output_get_2 "Emissive" (`self.EyeEmissive`))
          (`MaterialInstanceDynamic.SetScalarParameterValue` _output_get_2 "SceleraBrightness" (`self.EyeSceleraBrightness`)))
        (:`then_3`
          ;;[1 1 1] Cloth
          (`MeshComponent.SetVectorParameterValueOnMaterials` _outfitcomponents "ClothColourA" (`KismetMathLibrary.Conv_LinearColorToVector` (`KismetMathLibrary.Conv_ColorToLinearColor` (`self.ClothesColourA`))))
          (`MeshComponent.SetVectorParameterValueOnMaterials` _outfitcomponents "ClothColourB" (`KismetMathLibrary.Conv_LinearColorToVector` (`KismetMathLibrary.Conv_ColorToLinearColor` (`self.ClothesColourB`))))
          (`MeshComponent.SetVectorParameterValueOnMaterials` _outfitcomponents "ClothColourC" (`KismetMathLibrary.Conv_LinearColorToVector` (`KismetMathLibrary.Conv_ColorToLinearColor` (`self.ClothesColourC`))))
          (`MeshComponent.SetVectorParameterValueOnMaterials` _outfitcomponents "ClothColourD" (`KismetMathLibrary.Conv_LinearColorToVector` (`KismetMathLibrary.Conv_ColorToLinearColor` (`self.ClothesColourD`))))
          (`MeshComponent.SetVectorParameterValueOnMaterials` _outfitcomponents "ClothColourEmissive" (`KismetMathLibrary.Conv_LinearColorToVector` (`KismetMathLibrary.Conv_ColorToLinearColor` (`self.ClothesEmissiveColour`))))
          (`MeshComponent.SetScalarParameterValueOnMaterials` _outfitcomponents "ClothEmissiveAmount" (`self.ClothesEmissiveAmount`)))))))

(fn `ModularSetup`
  (locals (HairFrontBone :type Name :default "hair_front_root"))
  (bind _output_get (set `self.RootMesh` (`self.Mesh`)))
  (`SkinnedMeshComponent.SetLeaderPoseComponent` (`self.Torso`) _output_get false)
  (`SkinnedMeshComponent.SetLeaderPoseComponent` (`self.Legs`) _output_get false)
  (`SkinnedMeshComponent.SetLeaderPoseComponent` (`self.Hands`) _output_get false)
  (`SkinnedMeshComponent.SetLeaderPoseComponent` (`self.Feet_0`) _output_get false)
  (`SkinnedMeshComponent.SetLeaderPoseComponent` (`self.Belt`) _output_get false)
  (`SkinnedMeshComponent.SetLeaderPoseComponent` (`self.Accessory_C`) _output_get false)
  (`SkinnedMeshComponent.SetLeaderPoseComponent` (`self.Accessory_A`) _output_get false)
  (`SkinnedMeshComponent.SetLeaderPoseComponent` (`self.Accessory_B`) _output_get false)
  (`SkinnedMeshComponent.SetLeaderPoseComponent` (`self.BackPiece`) _output_get false)
  (`SkinnedMeshComponent.SetLeaderPoseComponent` (`self.Fringe`) _output_get false)
  (`SkinnedMeshComponent.SetLeaderPoseComponent` (`self.Hair`) _output_get false)
  (set `self.BodyComponents` (`|MakeArray` (`self.Mesh`) (`self.Torso`) (`self.Legs`) (`self.Hands`) (`self.Feet_0`)))
  (set `self.OutfitComponents` (`|MakeArray` (`self.Mesh`) (`self.Torso`) (`self.Legs`) (`self.Hands`) (`self.Feet_0`) (`self.Belt`) (`self.Accessory_C`) (`self.Accessory_A`) (`self.Accessory_B`)))
  (set `self.HairComponents` (`|MakeArray` (`self.Hair`) (`self.Fringe`) (`self.BackPiece`))))

(fn `SetMorphTarget`
  (params (S_Blendshape :type "/Game/XANDRA/_Master/Blueprints/Structs/S_Blendshape Structure") (Value :type "Float (double-precision)"))
  (bind (_positivename _negativename) (break `/Game/XANDRA/_Master/Blueprints/Structs/S_Blendshape` S_Blendshape))
  (bind _outfitcomponents (`self.OutfitComponents`))
  (if (> Value 0.001)
    (`SkeletalMeshComponent.SetMorphTarget` _outfitcomponents _positivename Value true)
    (`SkeletalMeshComponent.SetMorphTarget` _outfitcomponents _negativename 0.0 true)
    (else
      (`SkeletalMeshComponent.SetMorphTarget` _outfitcomponents _negativename (`KismetMathLibrary.Abs` Value) true)
      (`SkeletalMeshComponent.SetMorphTarget` _outfitcomponents _positivename 0.0 true)))
  (return))

(fn `SetSkinMasks`
  (`|ExecutionSequence`
    (:`then_0`
      (switch `/Game/XANDRA/_Master/Blueprints/Enums/E_EyeMakeup` (`self.EyeMakeupStyle`)
        (:`NewEnumerator3`
          (set `self.EyeMakeupMask` "/Game/XANDRA/_Master/Materials/General/Textures/T_Black_DIFF.T_Black_DIFF"))
        (:`NewEnumerator0`
          (set `self.EyeMakeupMask` "/Game/XANDRA/_Master/Materials/Skin/Textures/Masks/T_EyeMakeup_B_DIFF.T_EyeMakeup_B_DIFF"))
        (:`NewEnumerator1`
          (set `self.EyeMakeupMask` "/Game/XANDRA/_Master/Materials/Skin/Textures/Masks/T_EyeMakeup_A_DIFF.T_EyeMakeup_A_DIFF"))
        (:`NewEnumerator2`
          (set `self.EyeMakeupMask` "/Game/XANDRA/_Master/Materials/Skin/Textures/Masks/OLD/T_EyeMakeup_HF2_D_DIFF.T_EyeMakeup_HF2_D_DIFF"))
        (:`NewEnumerator4`
          (set `self.EyeMakeupMask` "/Game/XANDRA/_Master/Materials/Skin/Textures/Masks/T_EyeMakeup_D_MASK.T_EyeMakeup_D_MASK"))
        (:`NewEnumerator5`
          (set `self.EyeMakeupMask` "/Game/XANDRA/_Master/Materials/Skin/Textures/Masks/T_EyeMakeup_E.T_EyeMakeup_E"))))
    (:`then_1`
      (switch `/Game/XANDRA/_Master/Blueprints/Enums/E_BrowStyle` (`self.BrowStyle`)
        (:`NewEnumerator3`
          (set `self.BrowsMask` "/Game/XANDRA/_Master/Materials/General/Textures/T_Black_DIFF.T_Black_DIFF"))
        (:`NewEnumerator0`
          (set `self.BrowsMask` "/Game/XANDRA/_Master/Materials/Skin/Textures/Masks/T_Brows_A_MASK.T_Brows_A_MASK"))
        (:`NewEnumerator1`
          (set `self.BrowsMask` "/Game/XANDRA/_Master/Materials/Skin/Textures/Masks/T_Brows_B_MASK.T_Brows_B_MASK"))
        (:`NewEnumerator2`
          (set `self.BrowsMask` "/Game/XANDRA/_Master/Materials/Skin/Textures/Masks/T_Brows_C_DIFF.T_Brows_C_DIFF"))
        (:`NewEnumerator4`
          (set `self.BrowsMask` "/Game/XANDRA/_Master/Materials/Skin/Textures/Masks/T_Brows_D_DIFF.T_Brows_D_DIFF"))))
    (:`then_2`
      (switch `/Game/XANDRA/_Master/Blueprints/Enums/E_BlushStyle` (`self.BlushStyle`)
        (:`NewEnumerator3`
          (set `self.BlushMask` "/Game/XANDRA/_Master/Materials/General/Textures/T_Black_DIFF.T_Black_DIFF"))
        (:`NewEnumerator0`
          (set `self.BlushMask` "/Game/XANDRA/_Master/Materials/Skin/Textures/Masks/T_Blush_MASK.T_Blush_MASK"))
        (:`NewEnumerator1`
          (set `self.BlushMask` "/Game/XANDRA/_Master/Materials/Skin/Textures/Masks/T_Blush_B_MASK.T_Blush_B_MASK"))))))

(fn `UserConstructionScript`
  (`self.ModularSetup`)
  (`self.AnimationSetup`)
  (`self.CustomisationSetup`))